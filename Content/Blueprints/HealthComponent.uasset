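; Actor component that tracks health for its owner, starting at MaxHealth on BeginPlay.
; It subtracts damage from the owner's OnTakeAnyDamage and adds healing received through its OnHealthAdd dispatcher, capped at MaxHealth.
; Both changes broadcast OnHealthChanged and play a 2D sound, and damage that leaves health at zero or below also broadcasts OnHealthDepleted.
; The AddHealth handler ignores its IsMaxLife and NewMaxHealth inputs.
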(event `self.ReceiveBeginPlay`
  (set `self.Health` (`self.MaxHealth`))
  (add `Actor.OnTakeAnyDamage` (`self.GetOwner`) (delegate `TakeDamage`))
  (add `self.OnHealthAdd` (delegate `AddHealth`)))

(event `AddHealth` :!signature `self.OnHealthAdd`
  (params (`Health To Add` :type "Float (double-precision)") (`IsMaxLife?` :type Boolean) (`new max Health` :type "Float (double-precision)"))
  (bind _output_get (set `self.Health` (+ `Health To Add` (`self.Health`))))
  (if (>= _output_get (`self.MaxHealth`))
    (set `self.Health` (`self.MaxHealth`)))
  (`self.OnHealthChanged` _output_get (`self.MaxHealth`))
  (`GameplayStatics.PlaySound2D` "/Game/Blueprints/Sounds/life_pickup.life_pickup" 1.0 1.0 0.0 null null))

(event `TakeDamage`
  (params (DamagedActor :type "Actor Object Reference") (Damage :type "Float (single-precision)") (DamageType :type "DamageType Object Reference") (InstigatedBy :type "Controller Object Reference") (DamageCauser :type "Actor Object Reference"))
  (bind _output_get (set `self.Health` (- (`self.Health`) Damage)))
  (`self.OnHealthChanged` _output_get (`self.MaxHealth`))
  (`GameplayStatics.PlaySound2D` "/Game/Blueprints/Sounds/hurtPlayer_Cue.hurtPlayer_Cue" 1.0 1.0 0.0 null null)
  (if (<= (`self.Health`) 0.0)
    (`self.OnHealthDepleted`)))