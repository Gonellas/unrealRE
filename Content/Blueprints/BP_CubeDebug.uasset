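; BP_CubeDebug is a debug actor that reports jumps of third-person characters that have entered its trigger.
; When its Box is overlapped by a BP_ThirdPersonCharacter, it binds to that character's OnTPSCharacterJump dispatcher and prints the jumper's name on each jump.
; Nothing unbinds the event, and a second overlap binding on Cube is left unwired with an empty auto-generated function.
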(event `self.ReceiveBeginPlay`)

(event `self.Box.OnComponentBeginOverlap`
  (params (OverlappedComponent :type "PrimitiveComponent Object Reference") (OtherActor :type "Actor Object Reference") (OtherComp :type "PrimitiveComponent Object Reference") (OtherBodyIndex :type Integer) (bFromSweep :type Boolean) (SweepResult :type "HitResult Structure (by ref)"))
  (bind _asbp_third_person_character (cast `/Game/ThirdPerson/Blueprints/BP_ThirdPersonCharacter` OtherActor))
  (add `/Game/ThirdPerson/Blueprints/BP_ThirdPersonCharacter.OnTPSCharacterJump` _asbp_third_person_character (delegate `OnTPSCharacterJump_Event`)))

(event `OnTPSCharacterJump_Event`
  (params (Jumper :type "/Game/ThirdPerson/Blueprints/BP_ThirdPersonCharacter Object Reference"))
  (`KismetSystemLibrary.PrintString` (`KismetStringLibrary.Concat_StrStr` (`KismetSystemLibrary.GetDisplayName` Jumper) ": Jumped")))

(fn `BP_CubeDebug_AutoGenFunc`
  (params (OverlappedComponent :type "PrimitiveComponent Object Reference") (OtherActor :type "Actor Object Reference") (OtherComp :type "PrimitiveComponent Object Reference") (OtherBodyIndex :type Integer) (bFromSweep :type Boolean) (SweepResult :type "HitResult Structure (by ref)"))
  (return))

(fn `UserConstructionScript`)