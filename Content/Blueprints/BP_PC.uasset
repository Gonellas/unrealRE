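; BP_PC is a player controller that relays the possessed BP_ThirdPersonCharacter's life and coin changes to BP_HUD.
; On possess, it binds to the character's life-changed and coin-taken dispatchers, and the handlers call the HUD's display functions.
; Debug key J spawns a new character just ahead of the current pawn and possesses it, with no unbinding from the previous one.
; Debug key Tab only triggers an unconnected FlipFlop.
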(event Custom|OnLifeChanged_Event
  (params (NewCurrentLife :type Float%20%28double-precision%29) (NewMaxLife :type Float%20%28double-precision%29))
  (bind _asbp_hud (Utilities|Casting|CastToBP_HUD (HUD|GetHUD)))
  (Default|DisplayLife _asbp_hud NewCurrentLife NewMaxLife))

(event Custom|OnTakeCoins
  (params (NewCoins :type Integer))
  (bind _asbp_hud (Utilities|Casting|CastToBP_HUD (HUD|GetHUD)))
  (Default|DisplayCoins _asbp_hud NewCoins))

(event EventBeginPlay)

(event EventTick
  (params (DeltaSeconds :type Float%20%28single-precision%29)))

(event EventPossess
  (params (PossessedPawn :type Pawn%20Object%20Reference))
  (bind _asbp_third_person_character (Utilities|Casting|CastToBP_ThirdPersonCharacter PossessedPawn))
  (EventDispatchers|AssignOnLifeChanged _asbp_third_person_character (delegate Custom|OnLifeChanged_Event))
  (EventDispatchers|BindEventtoOnTakeCoin _asbp_third_person_character (delegate Custom|OnTakeCoins)))

(event Input|KeyboardEvents|DebugKeyTab
  (params (Key :type Key%20Structure :default "None") (ActionValue :type Input%20Action%20Value%20Structure))
  (:Pressed
    (Utilities|FlowControl|FlipFlop)))

(event Input|KeyboardEvents|DebugKeyJ
  (params (Key :type Key%20Structure :default "None") (ActionValue :type Input%20Action%20Value%20Structure))
  (bind _returnvalue (Pawn|GetControlledPawn))
  (:Pressed
    (bind _returnvalue_2 (Game|SpawnActorfromClass "/Game/ThirdPerson/Blueprints/BP_ThirdPersonCharacter.BP_ThirdPersonCharacter_C" (Math|Conversions|ToTransform(Vector) (+ (Transformation|GetActorLocation _returnvalue) (Transformation|GetActorForwardVector _returnvalue))) "Undefined" "MultiplyWithRoot" 0 0))
    (Pawn|Possess _returnvalue_2)))

(fn ConstructionScript)