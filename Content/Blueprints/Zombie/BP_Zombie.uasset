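; Melee zombie enemy that patrols waypoints, targets the sensed player and deals damage at close range.
; Stats and sounds come from the enemy data table.
; Tick checks player distance, runs a looping attack timer and advances waypoints, while AI perception feeds player targets to the Blackboard and adjusts walk speed.
; Health depletion triggers ragdoll, death sound, Blackboard dead flag, score award and delayed destruction.
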(event `GetWaypointTransform`
  (bind _output (`|GetArrayItem` (`self.Waypoints`) (`self.CurrentIndex`)))
  (if (> (`KismetArrayLibrary.Array_Length` (`self.Waypoints`)) 0)
    (bind _output_get (set `self.Desination` (`self.K2_GetActorLocation` _output)))
    (`BlackboardComponent.SetValueAsVector` (`AIBlueprintHelperLibrary.GetBlackboard` (`self.GetController`)) (`self.Destination`) _output_get)
    (if (<= (`self.GetDistanceTo` _output) 100.0)
      (`/Engine/EditorBlueprintResources/StandardMacros.IncrementInt` (`self.CurrentIndex`)
        (:`  `
          (if (>= (`self.CurrentIndex`) (`KismetArrayLibrary.Array_Length` (`self.Waypoints`)))
            (set `self.CurrentIndex` 0)))))))

(event `self.ReceiveBeginPlay`
  (bind _returnvalue (`|GetDataTableRow` "/Game/Blueprints/DT_Enemies.DT_Enemies" "Melee")
    (:`then`
      (set `self.EnemyData` _returnvalue))))

(event `CheckPlayerDistance`
  (bind (_enemydata_maxwalkspeed _enemydata_damage _enemydata_hurtsound _enemydata_diesound _enemydata_mindistancetoattackplayer) (break `/Game/Blueprints/Zombie/S_Enemy` (`self.EnemyData`)))
  (bind _asbp_third_person_character (cast `/Game/ThirdPerson/Blueprints/BP_ThirdPersonCharacter` (`GameplayStatics.GetPlayerCharacter` 0) :!pure true))
  ;[1 1 1] CHECK PLAYER DISTANCE
  (`/Engine/EditorBlueprintResources/StandardMacros.IsValid` _asbp_third_person_character
    (:`Is Valid`
      (if (<= (`self.GetDistanceTo` _asbp_third_person_character) _enemydata_mindistancetoattackplayer)
        (set `self.IsPlayerNear` true)
        (else
          (set `self.IsPlayerNear` false))))))

(event `self.ReceiveTick`
  (params (DeltaSeconds :type "Float (single-precision)"))
  (if (`self.Dead`)
    (set `self.IsPlayerNear` false)
    (else
      (`self.CheckPlayerDistance`)
      (`self.AttackAction`)
      (`self.GetWaypointTransform`))))

(event `self.HealthComponent.OnHealthDepleted`
  (bind (_enemydata_maxwalkspeed _enemydata_damage _enemydata_hurtsound _enemydata_diesound) (break `/Game/Blueprints/Zombie/S_Enemy` (`self.EnemyData`)))
  (`self.Ragdoll`)
  (`GameplayStatics.PlaySoundAtLocation` _enemydata_diesound (`self.K2_GetActorLocation`) (struct) 1.0 1.0 0.0 null null null null)
  (bind _output_get (set `self.Dead` true))
  (`BlackboardComponent.SetValueAsBool` (`AIBlueprintHelperLibrary.GetBlackboard` (`self.GetController`)) (`self.Dead Key`) _output_get)
  (`KismetSystemLibrary.K2_SetTimerDelegate` (delegate `DestroyActor`) 4.0)
  (`/Game/Blueprints/BP_ScoreComponent.AddScore` (`self.BP_ScoreComponent`) 100))

(event `DestroyActor`
  (`self.K2_DestroyActor`))

(event `self.HealthComponent.OnHealthChanged`
  (params (NewHealth :type "Float (double-precision)") (NewMaxHealth :type "Float (double-precision)"))
  (bind (_enemydata_maxwalkspeed _enemydata_damage _enemydata_hurtsound) (break `/Game/Blueprints/Zombie/S_Enemy` (`self.EnemyData`)))
  (`GameplayStatics.PlaySoundAtLocation` _enemydata_hurtsound (`self.K2_GetActorLocation`) (struct) 1.0 1.0 0.0 null null null null))

(event `AttackAction`
  ;[1 1 1] attack
  (if (`self.IsPlayerNear`)
    (if (not (`KismetSystemLibrary.K2_IsTimerActiveHandle` (`self.AttackTimer`)))
      (`self.Attack`)
      (bind _returnvalue (`KismetSystemLibrary.K2_SetTimerDelegate` (delegate `Attack`) 1.5 true))
      (set `self.AttackTimer` _returnvalue))
    (else
      (`KismetSystemLibrary.K2_ClearAndInvalidateTimerHandle` (`self.AttackTimer`)))))

(event `self.AIPerception.OnTargetPerceptionUpdated`
  (params (Actor :type "Actor Object Reference") (Stimulus :type "AIStimulus Structure"))
  (bind _enemydata_maxwalkspeed (break `/Game/Blueprints/Zombie/S_Enemy` (`self.EnemyData`)))
  ;[1 1 1] AI PERCEPTION
  ;[1 1 1] Sin esto los enemigos se targeteaban entre si
  (if (`self.ActorHasTag` Actor "Player")
    (`BlackboardComponent.SetValueAsObject` (`AIBlueprintHelperLibrary.GetBlackboard` (`self.GetController`)) (`self.Target Key`) (`KismetMathLibrary.SelectObject` Actor null (`.bSuccessfullySensed` (break `AIStimulus` Stimulus))))
    (set `CharacterMovementComponent.MaxWalkSpeed` 300.0 (`self.CharacterMovement`))
    (else
      (set `CharacterMovementComponent.MaxWalkSpeed` _enemydata_maxwalkspeed (`self.CharacterMovement`)))))

(event `Attack`
  ;[1 1 1] attack
  (if (not (`self.Dead`))
    (`GameplayStatics.ApplyDamage` (cast `/Game/ThirdPerson/Blueprints/BP_ThirdPersonCharacter` (`GameplayStatics.GetPlayerCharacter` 0) :!pure true) (`.Damage_8_1CE279094E316A7E4F58279C40117F9E` (break `/Game/Blueprints/Zombie/S_Enemy` (`self.EnemyData`))))))

(fn `Ragdoll`
  (`PrimitiveComponent.SetCollisionProfileName` (`self.Mesh`) "Ragdoll" true)
  (`PrimitiveComponent.SetSimulatePhysics` (`self.Mesh`) true)
  (`CharacterMovementComponent.DisableMovement` (`self.CharacterMovement`)))

(fn `UserConstructionScript`)