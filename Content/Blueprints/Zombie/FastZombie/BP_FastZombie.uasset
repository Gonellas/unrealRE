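; BP_FastZombie is the fast zombie enemy, configured from the "Fast" row of DT_Enemies.
; Each tick it cycles waypoint destinations into the Blackboard and checks player distance, stopping to deal damage on a looping timer when close.
; AI Perception writes the sensed player to the Blackboard target and adjusts walk speed.
; Health depletion triggers ragdoll, a death sound, score gain and delayed destruction.
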(event `self.ReceiveBeginPlay`
  (bind _returnvalue (`|GetDataTableRow` "/Game/Blueprints/DT_Enemies.DT_Enemies" "Fast")
    (:`then`
      (set `self.Data Enemy` _returnvalue))))

(event `GetWaypointTransform`
  (bind _output (`|GetArrayItem` (`self.WayPoints`) (`self.CurrentIndex`)))
  ;[1 1 1] GetWaypoints
  (if (> (`KismetArrayLibrary.Array_Length` (`self.WayPoints`)) 0)
    (bind _output_get (set `self.Destination` (`self.K2_GetActorLocation` _output)))
    (`BlackboardComponent.SetValueAsVector` (`AIBlueprintHelperLibrary.GetBlackboard` (`self.GetController`)) (`self.DestinationKey`) _output_get)
    (if (<= (`self.GetDistanceTo` _output) 100.0)
      (`/Engine/EditorBlueprintResources/StandardMacros.IncrementInt` (`self.CurrentIndex`)
        (:`  `
          (if (>= (`self.CurrentIndex`) (`KismetArrayLibrary.Array_Length` (`self.Waypoints`)))
            (set `self.CurrentIndex` 0)))))))

(event `self.ReceiveTick`
  (params (DeltaSeconds :type "Float (single-precision)"))
  (if (`self.Dead`)
    (set `self.IsPlayerNear` false)
    (else
      (`self.CheckPlayerDistance`)
      (`self.AttackAction`)
      (`self.GetWaypointTransform`))))

(event `CheckPlayerDistance`
  (bind (_data_enemy_maxwalkspeed _data_enemy_damage _data_enemy_hurtsound _data_enemy_diesound _data_enemy_mindistancetoattackplayer) (break `/Game/Blueprints/Zombie/S_Enemy` (`self.Data Enemy`)))
  (bind _asbp_third_person_character (cast `/Game/ThirdPerson/Blueprints/BP_ThirdPersonCharacter` (`GameplayStatics.GetPlayerCharacter` 0) :!pure true))
  ;[1 1 1] CheckPlayerDistance
  (`/Engine/EditorBlueprintResources/StandardMacros.IsValid` _asbp_third_person_character
    (:`Is Valid`
      (if (<= (`self.GetDistanceTo` _asbp_third_person_character) _data_enemy_mindistancetoattackplayer)
        (set `self.IsPlayerNear` true)
        (else
          (set `self.IsPlayerNear` false))))))

(event `self.HealthComponent.OnHealthDepleted`
  (bind (_data_enemy_maxwalkspeed _data_enemy_damage _data_enemy_hurtsound _data_enemy_diesound) (break `/Game/Blueprints/Zombie/S_Enemy` (`self.Data Enemy`)))
  (`self.RagDoll`)
  (`GameplayStatics.PlaySoundAtLocation` _data_enemy_diesound (`self.K2_GetActorLocation`) (struct) 1.0 1.0 0.0 null null null null)
  (set `self.Dead` true)
  (`KismetSystemLibrary.K2_SetTimerDelegate` (delegate `Destroy`) 4.0)
  (`/Game/Blueprints/BP_ScoreComponent.AddScore` (`self.BP_ScoreComponent`) 100))

(event `Destroy`
  (`self.K2_DestroyActor`))

(event `self.HealthComponent.OnHealthChanged`
  (params (NewHealth :type "Float (double-precision)") (NewMaxHealth :type "Float (double-precision)"))
  (bind (_data_enemy_maxwalkspeed _data_enemy_damage _data_enemy_hurtsound) (break `/Game/Blueprints/Zombie/S_Enemy` (`self.Data Enemy`)))
  (`GameplayStatics.PlaySoundAtLocation` _data_enemy_hurtsound (`self.K2_GetActorLocation`) (struct) 1.0 1.0 0.0 null null null null))

(event `AttackAction`
  ;[1 1 1] attack
  (if (`self.IsPlayerNear`)
    (if (`KismetSystemLibrary.K2_IsTimerActiveHandle` (`self.AttackTimer`))
      (set `CharacterMovementComponent.MaxWalkSpeed` 0.0 (`self.CharacterMovement`))
      (else
        (bind _returnvalue (`KismetSystemLibrary.K2_SetTimerDelegate` (delegate `Attack`) 0.7 true))
        (set `self.AttackTimer` _returnvalue)))
    (else
      (`KismetSystemLibrary.K2_ClearAndInvalidateTimerHandle` (`self.AttackTimer`))
      (set `CharacterMovementComponent.MaxWalkSpeed` 500.0 (`self.CharacterMovement`)))))

(event `self.AIPerception.OnTargetPerceptionUpdated`
  (params (Actor :type "Actor Object Reference") (Stimulus :type "AIStimulus Structure"))
  (bind _data_enemy_maxwalkspeed (break `/Game/Blueprints/Zombie/S_Enemy` (`self.Data Enemy`)))
  ;[1 1 1] AI PERCEPTION
  (if (`self.ActorHasTag` Actor "Player")
    (`BlackboardComponent.SetValueAsObject` (`AIBlueprintHelperLibrary.GetBlackboard` (`self.GetController`)) (`self.TargetKey`) (`KismetMathLibrary.SelectObject` Actor null (`.bSuccessfullySensed` (break `AIStimulus` Stimulus))))
    (set `CharacterMovementComponent.MaxWalkSpeed` 500.0 (`self.CharacterMovement`))
    (else
      (set `CharacterMovementComponent.MaxWalkSpeed` _data_enemy_maxwalkspeed (`self.CharacterMovement`)))))

(event `Attack`
  ;[1 1 1] attack
  (if (not (`self.Dead`))
    (`GameplayStatics.ApplyDamage` (cast `/Game/ThirdPerson/Blueprints/BP_ThirdPersonCharacter` (`GameplayStatics.GetPlayerCharacter` 0) :!pure true) (`.Damage_8_1CE279094E316A7E4F58279C40117F9E` (break `/Game/Blueprints/Zombie/S_Enemy` (`self.Data Enemy`))))))

(fn `RagDoll`
  (`PrimitiveComponent.SetCollisionProfileName` (`self.Mesh`) "Ragdoll" true)
  (`PrimitiveComponent.SetSimulatePhysics` (`self.Mesh`) true)
  (`CharacterMovementComponent.DisableMovement` (`self.CharacterMovement`)))

(fn `UserConstructionScript`)