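; Game instance for a coin-collecting game that saves and restores player progress across level loads.
; SaveGame writes the character's transform, coins and health, plus total score and current level name, to a BP_Savegame slot.
; MenuLoadGame sets a load flag, reads the save, opens its level and switches input to game-only.
; GameLoad separately applies the cached save to the character and refreshes score, health and coin displays or listeners.
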(event `MenuLoadGame`
  (bind _returnvalue (`GameplayStatics.GetPlayerController` 0))
  (set `self.LoadGame?` true)
  (bind _savedlevel (`self.LoadGame`))
  (`GameplayStatics.OpenLevel` (`KismetStringLibrary.Conv_StringToName` _savedlevel))
  (set `PlayerController.bShowMouseCursor` false _returnvalue)
  (`WidgetBlueprintLibrary.SetInputMode_GameOnly` _returnvalue))

(fn `GameLoad`
  (bind _character (`self.Character`))
  (bind _saveref (`self.SaveRef`))
  (bind _healthcomponent (`/Game/ThirdPerson/Blueprints/BP_ThirdPersonCharacter.HealthComponent` _character))
  (`Actor.K2_SetActorTransform` _character (`/Game/Blueprints/BP_Savegame.playerPos` _saveref) false false)
  (bind _output_get (set `/Game/Blueprints/HealthComponent.Health` (`/Game/Blueprints/BP_Savegame.SavedHealth` _saveref) _healthcomponent))
  (`/Game/Blueprints/HealthComponent.OnHealthChanged` _healthcomponent _output_get (`/Game/Blueprints/HealthComponent.MaxHealth` _healthcomponent))
  (bind _output_get_2 (set `self.TotalScore` (`/Game/Blueprints/BP_Savegame.SavedPoints` _saveref)))
  (bind _asbp_hud (cast `/Game/Blueprints/BP_HUD` (`PlayerController.GetHUD` (`GameplayStatics.GetPlayerController` 0))))
  (`/Game/Blueprints/BP_HUD.DisplayScore` _asbp_hud _output_get_2)
  (bind _output_get_3 (set `/Game/ThirdPerson/Blueprints/BP_ThirdPersonCharacter.Coins` (`/Game/Blueprints/BP_Savegame.SavedCoins` _saveref) _character))
  (`/Game/ThirdPerson/Blueprints/BP_ThirdPersonCharacter.OnTakeCoin` _character _output_get_3))

(fn `LoadGame`
  (returns (SavedLevel :type String))
  (bind _returnvalue (`GameplayStatics.LoadGameFromSlot` (`self.SlotNameSave`)))
  (bind _asbp_savegame (cast `/Game/Blueprints/BP_Savegame` _returnvalue))
  (bind _output_get (set `self.SaveRef` _asbp_savegame))
  (return (`/Game/Blueprints/BP_Savegame.SavedLevel` _output_get)))

(fn `SaveGame`
  (bind _saveref (`self.SaveRef`))
  (bind _returnvalue (`GameplayStatics.CreateSaveGameObject` "/Game/Blueprints/BP_Savegame.BP_Savegame_C"))
  (bind _output_get (set `self.SaveRef` _returnvalue))
  (set `/Game/Blueprints/BP_Savegame.playerPos` (`Actor.GetTransform` (`self.Character`)) _output_get)
  (set `/Game/Blueprints/BP_Savegame.SavedCoins` (`/Game/ThirdPerson/Blueprints/BP_ThirdPersonCharacter.Coins` (`self.Character`)) _saveref)
  (set `/Game/Blueprints/BP_Savegame.SavedPoints` (`self.TotalScore`) _saveref)
  (set `/Game/Blueprints/BP_Savegame.SavedHealth` (`/Game/Blueprints/HealthComponent.Health` (`/Game/ThirdPerson/Blueprints/BP_ThirdPersonCharacter.HealthComponent` (`self.Character`))) _saveref)
  (bind _returnvalue_2 (`GameplayStatics.GetCurrentLevelName` true))
  (set `/Game/Blueprints/BP_Savegame.SavedLevel` _returnvalue_2 (`self.SaveRef`))
  (`GameplayStatics.SaveGameToSlot` (`self.SaveRef`) (`self.SlotNameSave`)))