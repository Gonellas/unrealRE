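; BP_LifePU is a life pickup that adds its Life amount to a health value on sphere overlap, then destroys itself.
; The overlap shows a widget, adds a new health component to itself, clamps the increased Health, updates the HUD and adds it to the viewport.
; End overlap hides the widget.
; IsPlayer compares the actor to the player controller, but neither event uses its result.
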(event `self.Sphere.OnComponentBeginOverlap`
  (params (OverlappedComponent :type "PrimitiveComponent Object Reference") (OtherActor :type "Actor Object Reference") (OtherComp :type "PrimitiveComponent Object Reference") (OtherBodyIndex :type Integer) (bFromSweep :type Boolean) (SweepResult :type "HitResult Structure (by ref)"))
  (bind _hud (`self.HUD`))
  (`SceneComponent.SetVisibility` (`self.Widget`) true false)
  (`self.IsPlayer` OtherActor)
  (bind _returnvalue (`AddComponent|NODE_AddHealthComponent-0`))
  (bind _output_get (set `/Game/Blueprints/HealthComponent.Health` (`KismetMathLibrary.FClamp` (+ (`/Game/Blueprints/HealthComponent.Health` _returnvalue) (`self.Life`)) 0.0 100.0) _returnvalue))
  (`/Game/Blueprints/WBP_HUD.UpdateLife` _hud _output_get 0.0)
  (`UserWidget.AddToViewport` _hud 0)
  (`KismetSystemLibrary.PrintString` "sumo vida?")
  (`self.K2_DestroyActor`))

(event `self.Sphere.OnComponentEndOverlap`
  (params (OverlappedComponent :type "PrimitiveComponent Object Reference") (OtherActor :type "Actor Object Reference") (OtherComp :type "PrimitiveComponent Object Reference") (OtherBodyIndex :type Integer))
  (`SceneComponent.SetVisibility` (`self.Widget`) false false)
  (`self.IsPlayer` OtherActor))

(fn `IsPlayer`
  (params (Player :type "Actor Object Reference"))
  (returns (isPlayer :type Boolean))
  (if (== Player (`GameplayStatics.GetPlayerController` 0))
    (return true)
    (else
      (return false))))

(fn `UserConstructionScript`
  (locals (NewLocalVar :type "Transform Structure")))