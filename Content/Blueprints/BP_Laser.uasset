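; BP_Laser is a moving laser hazard that damages the player on contact.
; On BeginPlay, a timeline drives a swept vertical lerp of the actor between LaserUpPos and LaserDownPos, keeping its current X and Y.
; When its capsule begins overlapping an actor tagged Player, it sends that actor a TakeDamage message carrying its Damage value.
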(event `self.ReceiveBeginPlay`
  (bind (_returnvalue_x _returnvalue_y) (`KismetMathLibrary.BreakVector` (`self.K2_GetActorLocation`)))
  (bind (_laseruppos_x _laseruppos_y _laseruppos_z) (`KismetMathLibrary.BreakVector` (`self.LaserUpPos`)))
  (bind (_laserdownpos_x _laserdownpos_y _laserdownpos_z) (`KismetMathLibrary.BreakVector` (`self.LaserDownPos`)))
  (bind (_direction _laser_movement) (`Timeline|Timeline laser`)
    (:`Update`
      (`self.K2_SetActorLocation` (`KismetMathLibrary.VLerp` (`KismetMathLibrary.MakeVector` _returnvalue_x _returnvalue_y _laseruppos_z) (`KismetMathLibrary.MakeVector` _returnvalue_x _returnvalue_y _laserdownpos_z) _laser_movement) true))))

(event `self.Capsule.OnComponentBeginOverlap`
  (params (OverlappedComponent :type "PrimitiveComponent Object Reference") (OtherActor :type "Actor Object Reference") (OtherComp :type "PrimitiveComponent Object Reference") (OtherBodyIndex :type Integer) (bFromSweep :type Boolean) (SweepResult :type "HitResult Structure (by ref)"))
  (if (`self.ActorHasTag` OtherActor "Player")
    (message `/Game/Blueprints/Idamageable.TakeDamage` OtherActor (`self.Damage`))))

(fn `UserConstructionScript`)