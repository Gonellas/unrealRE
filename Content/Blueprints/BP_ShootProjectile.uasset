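; BP_ShootProjectile is an enemy shooter actor that fires bullets at the player while they are in range.
; Its Sphere overlap detects actors tagged Player, setting an in-range flag and starting or clearing a looping timer.
; Tick rotates the actor toward the player character while in range.
; Each timer shot spawns BP_bullet along the actor's forward vector and plays a drone shooting sound.
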(event `self.ReceiveTick`
  (params (DeltaSeconds :type "Float (single-precision)"))
  (if (`self.PlayerInRange`)
    (`self.LookAtPlayer`)))

(event `self.Sphere.OnComponentBeginOverlap`
  (params (OverlappedComponent :type "PrimitiveComponent Object Reference") (OtherActor :type "Actor Object Reference") (OtherComp :type "PrimitiveComponent Object Reference") (OtherBodyIndex :type Integer) (bFromSweep :type Boolean) (SweepResult :type "HitResult Structure (by ref)"))
  (if (`self.ActorHasTag` OtherActor "Player")
    (set `self.PlayerInRange` true)
    (bind _returnvalue (`KismetSystemLibrary.K2_SetTimerDelegate` (delegate `Shoot`) (`self.ShootCD`) true))
    (set `self.ShootTimer` _returnvalue)))

(event `Shoot`
  (`|SpawnActorFromClass` "/Game/Blueprints/BP_bullet.BP_bullet_C" (`KismetMathLibrary.MakeTransform` (`self.K2_GetActorLocation`) (`KismetMathLibrary.Conv_VectorToRotator` (`self.GetActorForwardVector`))) "Undefined" "MultiplyWithRoot" null null)
  (`GameplayStatics.PlaySound2D` "/Game/Blueprints/Sounds/DronShoot_Cue.DronShoot_Cue" 1.0 1.0 0.0 null null))

(event `self.Sphere.OnComponentEndOverlap`
  (params (OverlappedComponent :type "PrimitiveComponent Object Reference") (OtherActor :type "Actor Object Reference") (OtherComp :type "PrimitiveComponent Object Reference") (OtherBodyIndex :type Integer))
  (if (`self.ActorHasTag` OtherActor "Player")
    (set `self.PlayerInRange` false)
    (`KismetSystemLibrary.K2_ClearAndInvalidateTimerHandle` (`self.ShootTimer`))))

(event `LookAtPlayer`
  (`self.K2_SetActorRotation` (`KismetMathLibrary.FindLookAtRotation` (`self.K2_GetActorLocation`) (`self.K2_GetActorLocation` (cast `/Game/ThirdPerson/Blueprints/BP_ThirdPersonCharacter` (`GameplayStatics.GetPlayerCharacter` 0) :!pure true)))))

(fn `UserConstructionScript`)