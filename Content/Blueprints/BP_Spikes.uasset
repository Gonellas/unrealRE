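; Spike hazard Blueprint that deals repeated damage to an actor overlapping its Box.
; Begin overlap starts a looping one-second timer that applies Damage to that actor, with no tag filter and a single stored handle.
; End overlap clears that timer only for actors tagged Player.
; An AlreadyDamaged cooldown with a delayed reset exists but is disconnected and never runs.
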(event `self.Box.OnComponentBeginOverlap`
  (params (OverlappedComponent :type "PrimitiveComponent Object Reference") (OtherActor :type "Actor Object Reference") (OtherComp :type "PrimitiveComponent Object Reference") (OtherBodyIndex :type Integer) (bFromSweep :type Boolean) (SweepResult :type "HitResult Structure (by ref)"))
  (bind _returnvalue (`KismetSystemLibrary.K2_SetTimerDelegate` (delegate `ApplyDamage`) 1.0 true))
  (set `self.TimerDamage` _returnvalue))

(event `ApplyDamage`
  (`GameplayStatics.ApplyDamage` (stale `self.Box.OnComponentBeginOverlap` OtherActor) (`self.damage`)))

(event `Reset Already Damaged`
  (set `self.AlreadyDamaged` false))

(event `self.Box.OnComponentEndOverlap`
  (params (OverlappedComponent :type "PrimitiveComponent Object Reference") (OtherActor :type "Actor Object Reference") (OtherComp :type "PrimitiveComponent Object Reference") (OtherBodyIndex :type Integer))
  (if (`self.ActorHasTag` OtherActor "Player")
    (`KismetSystemLibrary.K2_ClearAndInvalidateTimerHandle` (`self.TimerDamage`))))

(fn `UserConstructionScript`)